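; BP_CrawlerHead is the head of a crawler enemy, with a cosmetic eye blink.
; On BeginPlay it starts a looping timer with a random interval, picked once per instance, and a wide initial start delay variance.
; Each tick of the timer briefly hides both eye components and their children, then shows them again after a short delay.
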(event Custom|Blink
  (Rendering|SetVisibility (Variables|Default|GetEye1) false true)
  (Rendering|SetVisibility (Variables|Default|GetEye2) false true)
  (Utilities|FlowControl|Delay 0.2)
  (Rendering|SetVisibility (Variables|Default|GetEye1) true true)
  (Rendering|SetVisibility (Variables|Default|GetEye2) true true))

(event EventBeginPlay
  (Utilities|Time|SetTimerbyEvent (delegate Custom|Blink) (Math|Random|RandomFloatinRange 4.0 8.0) true 0.0 2e+01))

(fn ConstructionScript)