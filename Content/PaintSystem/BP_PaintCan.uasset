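; BP_PaintCan is an interactable paint can that changes the brush used on the painting canvases.
; On Interact it finds every BP_Canvas in the level and sets its BrushTexture to the can's PaintColor.
; BeginPlay applies the can's color material to the sphere and creates an interact-button widget, which Hover and EndHover add to and remove from the viewport.
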(event EventHover
  ;[1 1 1] Hover
  (UserInterface|Viewport|AddtoViewport (Variables|Default|GetHoverHUD) 0))

(event EventEndHover
  ;[1 1 1] Hover
  (Widget|RemovefromParent (Variables|Default|GetHoverHUD)))

(event EventBeginPlay
  (Rendering|Material|SetMaterial (Variables|Default|GetSphere) 0 (Variables|Default|GetPaintCanColor))
  (bind _returnvalue (UserInterface|CreateWidget "/Game/Interact/W_InteractButton.W_InteractButton_C"))
  (Variables|Default|SetHoverHUD _returnvalue))

(event EventInteract
  (bind _outactors (Actor|GetAllActorsOfClass "/Game/PaintSystem/BP_Canvas.BP_Canvas_C"))
  (for _array_element _outactors
    (Variables|/Game/PaintSystem/BP_Canvas.BP_Canvas_C|SetBrush%20Texture _array_element (Variables|Default|GetPaint%20Color))))

(fn ConstructionScript)