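; BP_CanvasSlot is a paint-system slot that holds a BP_Canvas, optionally spawning a blank one and showing a spotlight.
; Player pickup and put-down events show or hide an empty slot, filtered by whether it accepts empty or painted canvases.
; Interacting attaches the held canvas and sets its pickup and paint permissions; picking it up again clears the slot.
; An empty slot that rejects painted canvases destroys itself when one is picked up.
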(event Custom|ShowCanvasSlot
  ;[1 1 1] OnPickup
  (Utilities|IsValid (Variables|Default|GetCanvas)
    (:Is%20Not%20Valid
      (bind _asbp_canvas (Utilities|Casting|CastToBP_Canvas (Variables|/Game/FirstPerson/Blueprints/BP_FirstPersonCharacter.BP_FirstPersonCharacter_C|GetItemHeld (Variables|Default|GetFPPlayerRef))))
      (if (Math|Boolean|NANDBoolean (not (Variables|Default|GetAcceptPaintedCanvas)) (Variables|/Game/PaintSystem/BP_Canvas.BP_Canvas_C|GetHasPaint _asbp_canvas))
        (if (or (Variables|Default|GetAcceptEmptyCanvas) (Variables|/Game/PaintSystem/BP_Canvas.BP_Canvas_C|GetHasPaint _asbp_canvas))
          (Rendering|SetVisibility (Variables|Default|GetCanvasSlot) true false)
          (Collision|SetCollisionEnabled (Variables|Default|GetCanvasSlot) "QueryAndPhysics"))
        (else
          ;[1 0 0] Delete Actor If there is no canvas in it, and it does not accept painted
          (Actor|DestroyActor))))))

(event Custom|HideCanvasSlot
  ;[1 1 1] PutDown
  (Rendering|SetVisibility (Variables|Default|GetCanvasSlot) false false)
  (Collision|SetCollisionEnabled (Variables|Default|GetCanvasSlot) "NoCollision"))

(event Custom|SetCanvasOptions
  (bind _canvas (Variables|Default|GetCanvas))
  ;[1 1 1] What options are available after placing in slot
  (Variables|/Game/PaintSystem/BP_Canvas.BP_Canvas_C|SetCanPickUpCanvas _canvas (Variables|Default|GetCanPickUpCanvas))
  (Variables|/Game/PaintSystem/BP_Canvas.BP_Canvas_C|SetCanInteract _canvas (Variables|Default|GetCanPaint)))

(event Custom|AddEmptyCanvas
  ;[1 1 1] Adds a blank canvas (best used at begin)
  (bind _returnvalue (Game|SpawnActorfromClass "/Game/PaintSystem/BP_Canvas.BP_Canvas_C" (Math|Transform|MakeTransform "0, 0, 0") "Undefined" "MultiplyWithRoot" 0 0))
  (CallFunction|AddCanvas _returnvalue))

(event Custom|Remove%20Canvas
  ;[1 1 1] Add Canvas
  (Variables|Default|SetCanvas 0))

(event Custom|AddCanvas
  (params (Canvas :type BP%20Canvas%20Object%20Reference))
  ;[1 1 1] Add Canvas
  (bind _output_get (Variables|Default|SetCanvas Canvas))
  (Transformation|DetachFromActor _output_get "KeepRelative" "KeepRelative" "KeepRelative")
  (Transformation|AttachComponentToComponent _output_get (Variables|Default|GetCanvasSlot) "None" "KeepRelative" "KeepRelative" "KeepRelative" true)
  (CallFunction|SetCanvasOptions)
  (EventDispatchers|BindEventtoPickedUp (Variables|Default|GetCanvas) (delegate Custom|Remove%20Canvas)))

(event EventInteract
  (bind _fpplayerref (Variables|Default|GetFPPlayerRef))
  (bind _itemheld (Variables|/Game/FirstPerson/Blueprints/BP_FirstPersonCharacter.BP_FirstPersonCharacter_C|GetItemHeld _fpplayerref))
  ;[1 1 1] Add Held Canvas
  (Utilities|IsValid _itemheld
    (:Is%20Valid
      (bind _asbp_canvas (Utilities|Casting|CastToBP_Canvas _itemheld))
      (if (Rendering|IsVisible (Variables|Default|GetCanvasSlot))
        (CallFunction|AddCanvas _asbp_canvas)
        (Default|PutDown (Variables|Default|GetFPPlayerRef))
        (CallFunction|HideCanvasSlot)))))

(event EventBeginPlay
  (bind _asbp_first_person_character (Utilities|Casting|CastToBP_FirstPersonCharacter (Game|Player|GetPlayerPawn 0)))
  (bind _output_get (Variables|Default|SetFPPlayerRef _asbp_first_person_character))
  (EventDispatchers|BindEventtoPickedUpItem _output_get (delegate Custom|ShowCanvasSlot))
  (EventDispatchers|BindEventtoPutDownItem _output_get (delegate Custom|HideCanvasSlot))
  (CallFunction|HideCanvasSlot)
  (Utilities|FlowControl|Sequence
    (:then_0
      (if (Variables|Default|GetOnBeginSpawnCanvas)
        (CallFunction|AddEmptyCanvas)))
    (:then_1
      (if (Variables|Default|GetHasDisplayLight)
        (Rendering|SetVisibility (Variables|Default|GetSpotLight) true false)
        (else
          (Rendering|SetVisibility (Variables|Default|GetSpotLight) false false))))))

(fn ConstructionScript)