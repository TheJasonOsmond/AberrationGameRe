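; Interactable hinged door that toggles open and closed, or plays a locked sound when CanOpen is false.
; A single Timeline drives the mesh yaw up to OpenAngle, reversing to close and playing the close sound when finished.
; ForceOpenDoor opens it regardless of the lock, and doors flagged IsOpen swing open on BeginPlay.
; Hover events add and remove an interact prompt widget created at start.
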(event Custom|ForceOpenDoor
  (if (not (Variables|Door|GetIsOpen))
    (Variables|Door|SetIsOpen true)
    (Audio|PlaySoundatLocation "/Game/OvaniSound/Sound/Objects/Wood_Rattling_001.Wood_Rattling_001" (Transformation|GetActorLocation) "0, 0, 0" 1.0 1.0 0.0 0 0 0 0)
    (bind _newtrack_0 (Timeline|Timeline Play)
      (:Update
        (Transformation|SetRelativeRotation (Variables|Default|GetSM_Door) (Math|Rotator|MakeRotator 0.0 0.0 (* _newtrack_0 (Variables|Door|GetOpenAngle))) false false))
      (:Finished
        ;[1 1 1] Close
        (if (not (Variables|Door|GetIsOpen))
          (Audio|PlaySoundatLocation "/Game/OvaniSound/Sound/Objects/Door/Plastic_Door_Close_001.Plastic_Door_Close_001" (Transformation|GetActorLocation) "0, 0, 0" 1.0 1.0 0.0 0 0 0 0))))))

(event EventBeginPlay
  ;[1 1 1] Open Door On Start
  (Utilities|FlowControl|Sequence
    (:then_0
      (if (Variables|Door|GetIsOpen)
        (bind _newtrack_0 (Timeline|Timeline Play)
          (:Update
            (Transformation|SetRelativeRotation (Variables|Default|GetSM_Door) (Math|Rotator|MakeRotator 0.0 0.0 (* _newtrack_0 (Variables|Door|GetOpenAngle))) false false))
          (:Finished
            ;[1 1 1] Close
            (if (not (Variables|Door|GetIsOpen))
              (Audio|PlaySoundatLocation "/Game/OvaniSound/Sound/Objects/Door/Plastic_Door_Close_001.Plastic_Door_Close_001" (Transformation|GetActorLocation) "0, 0, 0" 1.0 1.0 0.0 0 0 0 0))))))
    (:then_1
      (bind _returnvalue (UserInterface|CreateWidget "/Game/Interact/W_InteractButton.W_InteractButton_C"))
      (Variables|Default|SetInteractWidget _returnvalue))))

(event EventHover
  (UserInterface|Viewport|AddtoViewport (Variables|Default|GetInteractWidget) 0))

(event EventEndHover
  (Widget|RemovefromParent (Variables|Default|GetInteractWidget)))

(event EventInteract
  (if (Variables|Door|GetCanOpen)
    (if (Variables|Door|GetIsOpen)
      ;[1 1 1] Close
      (Variables|Door|SetIsOpen false)
      (bind _newtrack_0 (Timeline|Timeline Reverse)
        (:Update
          (Transformation|SetRelativeRotation (Variables|Default|GetSM_Door) (Math|Rotator|MakeRotator 0.0 0.0 (* _newtrack_0 (Variables|Door|GetOpenAngle))) false false))
        (:Finished
          ;[1 1 1] Close
          (if (not (Variables|Door|GetIsOpen))
            (Audio|PlaySoundatLocation "/Game/OvaniSound/Sound/Objects/Door/Plastic_Door_Close_001.Plastic_Door_Close_001" (Transformation|GetActorLocation) "0, 0, 0" 1.0 1.0 0.0 0 0 0 0))))
      (else
        ;[1 1 1] Open
        (Variables|Door|SetIsOpen true)
        (Audio|PlaySoundatLocation "/Game/OvaniSound/Sound/Objects/Door/Plastic_Door_Open_001.Plastic_Door_Open_001" (Transformation|GetActorLocation) "0, 0, 0" 1.0 1.0 0.0 0 0 0 0)
        (Timeline|Timeline Play)))
    (else
      ;[1 1 1] Locked Sound
      (Audio|PlaySoundatLocation "/Game/OvaniSound/Sound/Objects/Door/Metal_Door_Close_001.Metal_Door_Close_001" (Transformation|GetActorLocation) "0, 0, 0" 1.0 1.0 0.0 0 0 0 0))))

(fn ConstructionScript)