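; Light switch Blueprint that toggles a set of light actors in the game when interacted with.
; An Interact event calls UpdateLights, which flips the LightsOn flag and shows or hides every actor in the Lights array via SetActorHiddenInGame.
; BeginPlay runs the same toggle, so play starts in the opposite state to the LightsOn default.
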(event Custom|TurnOffLights
  ;[1 1 1] Turn Off
  (Variables|Default|SetLightsOn false)
  (for _array_element (Variables|Default|GetLights)
    (Rendering|SetActorHiddenInGame _array_element true)))

(event Custom|TurnOnLights
  ;[1 1 1] Turn On
  (Variables|Default|SetLightsOn true)
  (for _array_element (Variables|Default|GetLights)
    (Rendering|SetActorHiddenInGame _array_element false)))

(event Custom|UpdateLights
  ;[1 1 1] Update
  (if (Variables|Default|GetLightsOn)
    (CallFunction|TurnOffLights)
    (else
      (CallFunction|TurnonLights))))

(event EventInteract
  ;[1 1 1] Interact
  (CallFunction|UpdateLights))

(event EventBeginPlay
  ;[1 1 1] Begin
  (CallFunction|UpdateLights))

(fn ConstructionScript)