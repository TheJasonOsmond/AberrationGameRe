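; BPC_Interact is an interaction Blueprint that lets the player trigger interactable objects in the world.
; When IA_Interact starts, it runs a short complex line trace from the player camera along its forward vector against WorldDynamic and WorldStatic objects.
; If the hit actor implements BPI_Interactable, it calls InteractMessage on it, so each target defines its own response.
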(event Input|EnhancedActionEvents|EnhancedInputActionIA_Interact
  (params (ActionValue :type Boolean) (ElapsedSeconds :type Float%20%28double-precision%29) (TriggeredSeconds :type Float%20%28double-precision%29) (InputAction :type Input%20Action%20Object%20Reference :default "/Game/Interact/IA_Interact.IA_Interact"))
  (bind _returnvalue (Game|GetPlayerCameraManager 0))
  (bind _returnvalue_2 (Transformation|GetActorLocation _returnvalue))
  ;[1 1 1] Interact
  (:Started
    (bind _outhit (Collision|LineTraceForObjects _returnvalue_2 (+ _returnvalue_2 (* (Transformation|GetActorForwardVector _returnvalue) 3e+02)) (Utilities|Array|MakeArray "ObjectTypeQuery2" "ObjectTypeQuery1") true 0 "None" true "(R=1.000000,G=0.000000,B=0.000000,A=1.000000)" "(R=0.000000,G=1.000000,B=0.000000,A=1.000000)" 1.0))
    (if (Utilities|DoesObjectImplementInterface (.HitActor (Collision|BreakHitResult _outhit)) "/Game/Interact/BPI_Interactable.BPI_Interactable_C")
      (Class|BPIInteractable|Interact(Message) (.HitActor (Collision|BreakHitResult _outhit))))))