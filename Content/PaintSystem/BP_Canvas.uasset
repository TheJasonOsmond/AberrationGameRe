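; BP_Canvas is an interactable paintable canvas that switches the player into a fixed-position painting view with a crosshair HUD.
; On BeginPlay it creates a white render target, shown through a dynamic canvas material.
; Interact toggles painting, blending to the canvas camera with clamped look and halting player movement.
; Paint input traces from the camera, converts the hit to UV and draws the brush material into the render target.
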(event Custom|FinishPainting
  ;[1 1 1] Finish Painting
  (Variables|Default|SetisPainting false)
  (Game|Player|SetViewTargetwithBlend (Game|GetPlayerController 0) (Game|Player|GetPlayerPawn 0) (Variables|Camera|GetCameraBlendTime) "VTBlend_EaseInOut" (Variables|Camera|GetCameraBlendExp) false)
  (Pawn|Components|CharacterMovement|SetMovementMode (Variables|/Script/Engine.Character|GetCharacterMovement (Game|GetPlayerCharacter 0)) "MOVE_Walking" 0)
  (Input|DisableInput (Game|GetPlayerController 0) 0))

(event Custom|StartPainting
  ;[1 1 1] Start Painting
  (Pawn|Components|CharacterMovement|DisableMovement (Variables|/Script/Engine.Character|GetCharacterMovement (Game|GetPlayerCharacter 0)))
  (Game|Player|SetViewTargetwithBlend (Game|GetPlayerController 0) self (Variables|Camera|GetCameraBlendTime) "VTBlend_EaseInOut" (Variables|Camera|GetCameraBlendExp) false)
  (UserInterface|Viewport|AddtoViewport (Variables|Default|GetPaintHUD) 0)
  (Input|EnableInput (Game|GetPlayerController 0)))

(event Input|EnhancedActionEvents|EnhancedInputActionIA_Paint
  (params (ActionValue :type Float%20%28double-precision%29) (ElapsedSeconds :type Float%20%28double-precision%29) (TriggeredSeconds :type Float%20%28double-precision%29) (InputAction :type Input%20Action%20Object%20Reference :default "/Game/PaintSystem/Input/IA_Paint.IA_Paint"))
  (bind _returnvalue (Game|GetPlayerCameraManager 0))
  (bind _returnvalue_2 (Transformation|GetActorLocation _returnvalue))
  ;[1 1 1] Paint
  (:Triggered
    (if (== ActionValue 1.0)
      (if (Variables|Default|GetisPainting)
        (bind _outhit (Collision|LineTraceByChannel _returnvalue_2 (+ _returnvalue_2 (* (Transformation|GetActorForwardVector _returnvalue) (* (|CollapseGraph) 2e+02))) "TraceTypeQuery1" true 0 "None" false))
        (bind _asbp_canvas (Utilities|Casting|CastToBP_Canvas (.HitActor (Collision|BreakHitResult _outhit))))
        (CallFunction|DrawBrush _asbp_canvas (Variables|Default|GetBrush%20Texture) (Variables|Default|GetBrushSize) (.UV (Class|GameplayStatics|FindCollisionUV _outhit)))))))

(event Input|EnhancedActionEvents|EnhancedInputActionIA_Look
  (params (ActionValue :type Vector%202D%20Structure) (ElapsedSeconds :type Float%20%28double-precision%29) (TriggeredSeconds :type Float%20%28double-precision%29) (InputAction :type Input%20Action%20Object%20Reference :default "/Game/FirstPerson/Input/Actions/IA_Look.IA_Look"))
  (bind _camera (Variables|Default|GetCamera))
  (bind _camera_2 (Variables|Default|GetCamera))
  (bind _returnvalue (Transformation|GetWorldRotation _camera_2))
  ;[1 1 1] Look Controls
  (:Triggered
    (Transformation|AddWorldRotation _camera (Math|Rotator|MakeRotator 0.0 0.0 (Class|KismetMathLibrary|ClampAxis (* (.x ActionValue) 1.0))) false false)
    (Transformation|AddLocalRotation _camera (Math|Rotator|MakeRotator 0.0 (Class|KismetMathLibrary|ClampAxis (* (.y ActionValue) -1.0)) 0.0) false false)
    (Transformation|SetWorldRotation _camera_2 (Math|Rotator|MakeRotator 0.0 (Math|Float|ClampAngle (.pitch _returnvalue) (Variables|Camera|GetCameraLowerBound) (Variables|Camera|GetCameraUpperBound)) (Math|Float|ClampAngle (.yaw _returnvalue) (Variables|Camera|GetCameraLeftBound) (Variables|Camera|GetCameraRightBound))) false false)))

(event EventBeginPlay
  ;[1 1 1] BeginPlay
  (Utilities|FlowControl|Sequence
    (:then_0
      (bind _returnvalue (Rendering|CreateRenderTarget2D 1024 1024 "RTF_RGBA16f"))
      (bind _output_get (Variables|Default|SetRenderTarget _returnvalue))
      (Rendering|ClearRenderTarget2D _output_get "(R=1.000000,G=1.000000,B=1.000000,A=1.000000)"))
    (:then_1
      (bind _returnvalue_2 (Rendering|Material|CreateDynamicMaterialInstance "/Game/PaintSystem/M_Canvas.M_Canvas" "None" "None" :!class /Script/Engine.KismetMaterialLibrary))
      (Rendering|Material|SetTextureParameterValue _returnvalue_2 (Variables|Default|GetCanvasTextureParameter) (Variables|Default|GetRenderTarget))
      (Rendering|Material|SetMaterial (Variables|Default|GetCanvas) 0 _returnvalue_2))
    (:then_2
      (bind _returnvalue_3 (Rendering|Material|CreateDynamicMaterialInstance "/Game/PaintSystem/M_Brush.M_Brush" "None" "None" :!class /Script/Engine.KismetMaterialLibrary))
      (Variables|Default|SetBrushMaterial _returnvalue_3))
    (:then_3
      (bind _returnvalue_4 (UserInterface|CreateWidget "/Game/UI/W_CrossHair.W_CrossHair_C"))
      (Variables|Default|SetPaintHUD _returnvalue_4))))

(event EventInteract
  ;[1 1 1] Interact
  (if (Variables|Default|GetisPainting)
    (CallFunction|FinishPainting)
    (else
      (Variables|Default|SetisPainting true)
      (CallFunction|StartPainting))))

(fn ConstructionScript)

(fn DrawBrush
  (params (BrushTexture :type Texture%202D%20Object%20Reference) (BrushSize :type Float%20%28double-precision%29) (DrawLocation :type Vector%202D%20Structure))
  (Utilities|FlowControl|Sequence
    (:then_0
      (Rendering|Material|SetTextureParameterValue (Variables|Default|GetBrushMaterial) (Variables|Default|GetBrushTextureParameter) BrushTexture))
    (:then_1
      (bind (_canvas _size _context) (Rendering|BeginDrawCanvastoRenderTarget (Variables|Default|GetRenderTarget)))
      (Canvas|DrawMaterial :self _canvas :RenderMaterial (Variables|Default|GetBrushMaterial) :ScreenPosition (- (* _size DrawLocation) (/ BrushSize 2.0)) :ScreenSize (Math|Vector2D|MakeVector2D BrushSize BrushSize) :CoordinateSize "(X=1.000000,Y=1.000000)" :PivotPoint "(X=0.500000,Y=0.500000)")
      (Rendering|EndDrawCanvastoRenderTarget _context))))