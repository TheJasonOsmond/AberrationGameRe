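; BP_SceneController runs scripted horror scenes triggered when the player starts painting on a canvas.
; It binds to every BP_Canvas on BeginPlay, then unbinds the active one and picks a scene by the PaintScene counter.
; The first scene is a timed placeholder.
; The second locks canvas interaction while a delay-driven collapsed graph cuts lights, opens the art room door, moves the enemy in, silences the radio and plays sounds.
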(event Custom|StartPaintScene
  (bind _paintscene (Variables|Default|GetPaintScene))
  ;[1 1 1] StartNextPaintScene
  (CallFunction|GetCurrentCanvas)
  (EventDispatchers|UnbindEventfromStartedPainting (Variables|Default|GetCurrentCanvas) (delegate Custom|StartPaintScene))
  (if (== _paintscene 0)
    (CallFunction|PaintScene0)
    (elif (== _paintscene 1)
      (CallFunction|PaintScene1))))

(event Custom|DisableInteract
  ;[1 1 1] Toggle Interact
  (Variables|/Game/PaintSystem/BP_Canvas.BP_Canvas_C|SetCanInteract (Variables|Default|GetCurrentCanvas) false))

(event Custom|GetCurrentCanvas
  ;[1 1 1] Get Active Canvas
  (bind _array_element (Utilities|Array|ForEachLoopwithBreak (Variables|Default|GetCanvasList) :!label _label)
    (:LoopBody
      (if (Variables|/Game/PaintSystem/BP_Canvas.BP_Canvas_C|GetisPainting _array_element)
        (Variables|Default|SetCurrentCanvas _array_element)
        (goto _label Break)))))

(event Custom|EnableInteract
  ;[1 1 1] Toggle Interact
  (Variables|/Game/PaintSystem/BP_Canvas.BP_Canvas_C|SetCanInteract (Variables|Default|GetCurrentCanvas) true))

(event Custom|PaintScene1
  ;[1 1 1] Scene 1
  (CallFunction|DisableInteract)
  (|CollapseGraph
    (:Completed
      (CallFunction|EnableInteract)
      (Math|Integer|IncrementInt (Variables|Default|GetPaintScene)))))

(event Custom|PaintScene0
  ;[1 1 1] Scene 0
  (Math|Integer|IncrementInt (Variables|Default|GetPaintScene)
    (:%20%20
      (Development|PrintString "SCENE 0")
      (Utilities|FlowControl|Delay 5.0)
      (CallFunction|EnableInteract)
      (Development|PrintString "SCENE 0 FINISHED"))))

(event EventBeginPlay
  ;[1 1 1] On Begin: Bind To All Canvas'
  (Utilities|FlowControl|DelayUntilNextTick)
  (bind _outactors (Actor|GetAllActorsOfClass "/Game/PaintSystem/BP_Canvas.BP_Canvas_C"))
  (bind _output_get (Variables|Default|SetCanvasList _outactors))
  (for _array_element _output_get
    (EventDispatchers|BindEventtoStartedPainting _array_element (EventDispatchers|CreateEvent :!event Custom|StartPaintScene))))

(fn ConstructionScript)