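; Scene controller that runs staged horror sequences as the player starts painting on canvases, ending in an end menu.
; It binds to existing and respawned canvases, then uses a PaintScene counter to pick each scene, locking canvas interaction during timed events.
; Scene 1 stages door, light, radio and enemy scares; Scene 2 runs looping sound timers until painting finishes.
; Display-slot painting events are bound between scenes, finally triggering the paused end menu.
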(event Custom|CallRandomSound
  (bind _crawlervoices (Variables|Default|GetCrawlerVoices))
  ;[1 1 1] Call Random Sound
  (bind _result (Math|Integer|DecrementInt (Utilities|Array|Length _crawlervoices))
    (:%20%20
      (CallFunction|PlayRandCeilingLocation (Utilities|Array|Get(acopy) _crawlervoices (Math|Random|RandomIntegerinRange 0 _result))))))

(event Custom|DisableInteract
  ;[1 1 1] Toggle Interact
  (Variables|/Game/PaintSystem/BP_Canvas.BP_Canvas_C|SetCanInteract (Variables|Default|GetCurrentCanvas) false))

(event Custom|StartPaintScene
  (bind _paintscene (Variables|Default|GetPaintScene))
  ;[1 1 1] StartNextPaintScene
  (CallFunction|GetCurrentCanvas)
  (EventDispatchers|UnbindEventfromStartedPainting (Variables|Default|GetCurrentCanvas) (delegate Custom|StartPaintScene))
  (if (== _paintscene 0)
    (CallFunction|PaintScene0)
    (elif (== _paintscene 1)
      (CallFunction|PaintScene1)
      (elif (== _paintscene 2)
        (CallFunction|PaintScene2)
        (else
          (Variables|Default|SetLoopingScene2 true)
          (CallFunction|PaintScene2))))))

(event Custom|EndGame
  (bind _returnvalue (Game|GetPlayerController 0))
  ;[1 1 1] End Game
  (Utilities|FlowControl|DoOnce false
    (:Completed
      (bind _returnvalue_2 (UserInterface|CreateWidget "/Game/UI/W_EndMenu.W_EndMenu_C"))
      (Game|SetGamePaused true)
      (Input|SetInputModeUIOnly _returnvalue _returnvalue_2 "DoNotLock" false)
      (Variables|/Script/Engine.PlayerController|SetbShowMouseCursor _returnvalue true)
      (bind _asbp_first_person_character (Utilities|Casting|CastToBP_FirstPersonCharacter (Game|GetPlayerCharacter 0)))
      (Variables|/Game/FirstPerson/Blueprints/BP_FirstPersonCharacter.BP_FirstPersonCharacter_C|SetIsPausedMenuOpen _asbp_first_person_character true)
      (UserInterface|Viewport|AddtoViewport _returnvalue_2 0)
      (Development|PrintString "Exit Menu Added"))))

(event Custom|GetCurrentCanvas
  ;[1 1 1] Get Active Canvas
  (bind _array_element (Utilities|Array|ForEachLoopwithBreak (Variables|Default|GetCanvasList) :!label _label)
    (:LoopBody
      (if (Variables|/Game/PaintSystem/BP_Canvas.BP_Canvas_C|GetisPainting _array_element)
        (Variables|Default|SetCurrentCanvas _array_element)
        (goto _label Break)))))

(event Custom|EnableInteract
  (bind _currentcanvas (Variables|Default|GetCurrentCanvas))
  ;[1 1 1] Toggle Interact
  (Variables|/Game/PaintSystem/BP_Canvas.BP_Canvas_C|SetCanInteract _currentcanvas true)
  (Default|ShowFinishText _currentcanvas))

(event Custom|PaintScene1
  ;[1 1 1] Scene 1
  (CallFunction|DisableInteract)
  (|Scene1
    (:Completed
      (CallFunction|EnableInteract)
      (Math|Integer|IncrementInt (Variables|Default|GetPaintScene)
        (:%20%20
          (bind _outactors (Actor|GetAllActorsOfClass "/Game/PaintSystem/BP_CanvasSlot.BP_CanvasSlot_C"))
          (bind _array_element (Utilities|Array|ForEachLoopwithBreak _outactors)
            (:LoopBody
              (if (not (Variables|/Game/PaintSystem/BP_CanvasSlot.BP_CanvasSlot_C|GetCanPickUpCanvas _array_element))
                (Utilities|Array|Add (Variables|Default|GetCanvasDisplaySlots) _array_element)
                (EventDispatchers|BindEventtoPaintingAdded _array_element (EventDispatchers|CreateEvent :!event Custom|PrepScene2))))))))))

(event Custom|PaintScene0
  ;[1 1 1] Scene 0
  (Math|Integer|IncrementInt (Variables|Default|GetPaintScene)
    (:%20%20
      (Development|PrintString "SCENE 0")
      (CallFunction|DisableInteract)
      (Utilities|FlowControl|Delay 5.0)
      (CallFunction|EnableInteract)
      (Development|PrintString "SCENE 0 FINISHED"))))

(event Custom|AddCanvasToWatch
  ;[1 1 1] On Begin: Bind To All Canvas'
  (Utilities|IsValid (stale EventBeginPlay _array_element_2)
    (:Is%20Valid
      (EventDispatchers|BindEventtoStartedPainting (Variables|/Game/PaintSystem/BP_CanvasSlot.BP_CanvasSlot_C|GetCanvas (stale EventBeginPlay _array_element_2)) (EventDispatchers|CreateEvent :!event Custom|StartPaintScene)))
    (:Is%20Not%20Valid
      (Development|PrintString "Not a Valid Canvas Slot"))))

(event Custom|PrepScene2
  ;[1 1 1] Scene 2
  (Actor|DestroyActor (Variables|Default|GetCeiling))
  (EventDispatchers|UnbindallEventsfromPaintingAdded (Variables|Default|GetCanvasDisplaySlots))
  (Actor|DestroyActor (Variables|Default|GetRadio)))

(event Custom|PaintScene2
  (bind _loopingscene2 (Variables|Default|GetLoopingScene2))
  (bind _returnvalue (not _loopingscene2))
  ;[1 1 1] Scene 2
  (if _returnvalue
    (CallFunction|DisableInteract))
  (|Scene2)
  (if _returnvalue
    (Utilities|FlowControl|Delay 45.0)
    (CallFunction|EnableInteract)
    (Math|Integer|IncrementInt (Variables|Default|GetPaintScene)
      (:%20%20
        ;[1 1 1] End Game
        (bind _outactors (Actor|GetAllActorsOfClass "/Game/PaintSystem/BP_CanvasSlot.BP_CanvasSlot_C"))
        (bind _array_element (Utilities|Array|ForEachLoopwithBreak _outactors)
          (:LoopBody
            (if (not (Variables|/Game/PaintSystem/BP_CanvasSlot.BP_CanvasSlot_C|GetCanPickUpCanvas _array_element))
              (Utilities|Array|Add (Variables|Default|GetCanvasDisplaySlots) _array_element)
              (EventDispatchers|BindEventtoPaintingAdded _array_element (delegate Custom|EndGame))
              (Development|PrintString "Slots Binded"))))))
    (else
      (Default|ShowFinishText (Variables|Default|GetCurrentCanvas)))))

(event Custom|PlayRandCeilingLocation
  (params (Sound :type Sound%20Base%20Object%20Reference))
  ;[1 1 1] Plays a Sound at a Random Crawler Head In Scene 2
  (bind _outactors (Actor|GetAllActorsOfClasswithTag "/Game/Enemies/BP_CrawlerHead.BP_CrawlerHead_C" "Scene2"))
  (bind _result (Math|Integer|DecrementInt (Utilities|Array|Length _outactors))
    (:%20%20
      (Audio|PlaySoundatLocation Sound (Transformation|GetActorLocation (Utilities|Array|Get(acopy) _outactors (Math|Random|RandomIntegerinRange 0 _result))) "0, 0, 0" 1.0 1.0 0.0 0 0 0 0))))

(event EventBeginPlay
  ;[1 1 1] On Begin: Bind To All Canvas'
  (Utilities|FlowControl|DelayUntilNextTick)
  (bind _outactors (Actor|GetAllActorsOfClass "/Game/PaintSystem/BP_Canvas.BP_Canvas_C"))
  (bind _output_get (Variables|Default|SetCanvasList _outactors))
  (for _array_element _output_get
    (EventDispatchers|BindEventtoStartedPainting _array_element (EventDispatchers|CreateEvent :!event Custom|StartPaintScene))
    (bind _outactors_2 (Actor|GetAllActorsOfClass "/Game/PaintSystem/BP_CanvasSlot.BP_CanvasSlot_C"))
    (for _array_element_2 _outactors_2
      (if (Variables|/Game/PaintSystem/BP_CanvasSlot.BP_CanvasSlot_C|GetIsRespawning _array_element_2)
        (EventDispatchers|BindEventtoRespawnedCanvas _array_element_2 (delegate Custom|AddCanvasToWatch))))))

(fn ConstructionScript)

(event Custom|StopSounds
  ;[1 1 1] Stop and Unbind Timers
  (Utilities|Time|ClearandInvalidateTimerbyHandle (stale _returnvalue))
  (Utilities|Time|ClearandInvalidateTimerbyHandle (stale _returnvalue))
  (EventDispatchers|UnbindEventfromFinishedPainting (Variables|Default|GetCurrentCanvas) (delegate Custom|StopSounds)))