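; BP_Light is a switchable point light actor that applies its Intensity variable to the light on BeginPlay.
; TurnOn and TurnOff toggle the light's visibility and play a switch sound at its location.
; Flicker runs a looping timer at a short random interval that alternates off and on through a FlipFlop, then clears it after the given Duration and leaves the light on.
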(event Custom|TurnOff
  (bind _pointlight (Variables|Default|GetPointLight))
  (Rendering|SetVisibility _pointlight false false)
  (Audio|PlaySoundatLocation "/Game/OvaniSound/Sound/Lights/Light_Switch_Off_A.Light_Switch_Off_A" (Transformation|GetWorldLocation _pointlight) "0, 0, 0" 1.0 1.0 0.0 0 0 0 0))

(event Custom|Turn%20On
  (bind _pointlight (Variables|Default|GetPointLight))
  (Rendering|SetVisibility _pointlight true false)
  (Audio|PlaySoundatLocation "/Game/OvaniSound/Sound/Lights/Lamp_Switch_On_B.Lamp_Switch_On_B" (Transformation|GetWorldLocation _pointlight) "0, 0, 0" 1.0 1.0 0.0 0 0 0 0))

(event Custom|Flicker
  (params (Duration :type Float%20%28double-precision%29) (DelayVariance :type Float%20%28double-precision%29))
  (bind _returnvalue (Utilities|Time|SetTimerbyEvent (delegate Custom|FlickerFlipFlop) (Math|Random|RandomFloatinRange 0.05 0.1) true 0.0 DelayVariance))
  (Utilities|FlowControl|Delay Duration)
  (Utilities|Time|ClearandInvalidateTimerbyHandle _returnvalue)
  (CallFunction|Turnon))

(event Custom|FlickerFlipFlop
  (Utilities|FlowControl|FlipFlop
    (:A
      (CallFunction|TurnOff))
    (:B
      (CallFunction|Turnon))))

(event EventBeginPlay
  (Rendering|Components|Light|SetIntensity (Variables|Default|GetPointLight) (Variables|Default|GetIntensity)))

(fn ConstructionScript)