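; BP_Radio is an interactable radio that plays tracks from a media playlist.
; On BeginPlay it opens the playlist on its Media Player, then pauses after a short delay so it starts paused.
; Interact alternates between play and pause through a FlipFlop, and InteractAlt skips to the next playlist entry.
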(event Custom|ToggleRadio
  (bind _mediaplayer (Variables|Default|GetMediaPlayer))
  (Utilities|FlowControl|FlipFlop
    (:A
      (Media|MediaPlayer|Play _mediaplayer :!class /Script/MediaAssets.MediaPlayer))
    (:B
      (Sequencer|Player|Pause _mediaplayer))))

(event EventBeginPlay
  (Class|MediaPlayer|OpenPlaylist (Variables|Default|GetMediaPlayer) "/Game/Radio/Tracks/MP_RadioPlaylist.MP_RadioPlaylist")
  (Utilities|FlowControl|Delay 0.2)
  (Sequencer|Player|Pause (Variables|Default|GetMediaPlayer)))

(event EventInteract
  (CallFunction|ToggleRadio))

(event EventInteractAlt
  (Class|MediaPlayer|Next (Variables|Default|GetMediaPlayer)))

(fn ConstructionScript)